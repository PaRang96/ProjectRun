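; BP_RunPlayerState is the player state for the Run game mode, holding a player's name and point score.
; SetName assigns the name and AddPoint increments the score.
; RepNotify functions on both variables pass the replicated values to name and point dispatchers, so listeners can react to changes without polling.
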(fn `AddPoint`
  (params (Point :type Integer))
  (set `self.Point` (+ Point (`self.Point`))))

(fn `OnRep_Name`
  (`self.NameDispatcher` (`self.Name`)))

(fn `OnRep_Point`
  (`self.PointDispatcher` (`self.Point`)))

(fn `SetName`
  (params (Name :type String))
  (set `self.Name` Name))

(fn `UserConstructionScript`)