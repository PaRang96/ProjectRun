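; BP_RunGameMode is the game mode Blueprint for the Run game, handling rank-based scoring.
; AddRankScores walks PlayerRanking and calls AddPoint on each BP_RunPlayerState, with points falling linearly by finishing position.
; The event graph also holds logic to disable input for every player controller, but it is disconnected and never runs.
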(fn `AddRankScores`
  (for (_array_element _array_index) (`self.PlayerRanking`)
    (bind _asbp_run_player_state (cast `/Game/ProjectRun/GameMode/RunGame/BP_RunPlayerState` (`Controller.PlayerState` _array_element)))
    (`/Game/ProjectRun/GameMode/RunGame/BP_RunPlayerState.AddPoint` _asbp_run_player_state (* (- 3 _array_index) 100))))

(fn `UserConstructionScript`)